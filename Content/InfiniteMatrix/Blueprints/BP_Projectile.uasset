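; BP_Projectile is a projectile that flies along world +X and scales its speed with the player's progress.
; Each Tick reads Score and ForwardSpeed from the BP_Player pawn and moves the actor by a frame-rate independent offset, staying faster than the player's forward speed.
; It destroys itself on any actor overlap or when its short lifespan, set at BeginPlay, runs out.
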(event EventBeginPlay
  (Actor|SetLifeSpan 5.0))

(event Collision|EventActorBeginOverlap
  (params (OtherActor :type Actor%20Object%20Reference))
  (Actor|DestroyActor))

(event EventTick
  (params (DeltaSeconds :type Float%20%28single-precision%29))
  (bind _asbp_player (Utilities|Casting|CastToBP_Player (Game|Player|GetPlayerPawn 0)))
  (Transformation|AddActorWorldOffset (Math|Vector|MakeVector (* (+ (+ (* (Variables|/Game/InfiniteMatrix/Blueprints/BP_Player.BP_Player_C|GetScore _asbp_player) 30) (Variables|/Game/InfiniteMatrix/Blueprints/BP_Player.BP_Player_C|GetForwardSpeed _asbp_player)) 1e+03) DeltaSeconds) 0.0 0.0)))

(fn ConstructionScript)